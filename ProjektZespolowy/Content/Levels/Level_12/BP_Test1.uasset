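; BP_Test1 is a Level 12 interactable actor that opens and toggles the WB_Level12_Test1 screen widget.
; It extends the parent's BeginInteraction, creating the widget on first use, caching it as Level12Part1, and showing it with the mouse cursor.
; While the cached widget is valid, a FlipFlop alternates further interactions between hiding and showing both widget and cursor, starting with hide.
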(event `self.BeginInteraction`
  (bind _returnvalue (`GameplayStatics.GetPlayerController` 0))
  (bind _level12part1 (`self.Level12Part1`))
  (`parent.BeginInteraction`)
  (`self.Level12Part1`
    (:`then`
      (`/Engine/EditorBlueprintResources/StandardMacros.FlipFlop`
        (:`A`
          (`Widget.SetVisibility` _level12part1 "Hidden")
          (set `PlayerController.bShowMouseCursor` false _returnvalue))
        (:`B`
          (`Widget.SetVisibility` _level12part1 "Visible")
          (set `PlayerController.bShowMouseCursor` true _returnvalue))))
    (:`else`
      (bind _returnvalue_2 (`|CreateWidget` "/Game/LevelWidgets/Level12/WB_Level12_Test1.WB_Level12_Test1_C" (`GameplayStatics.GetPlayerController` 0)))
      (bind _output_get (set `self.Level12Part1` _returnvalue_2))
      (`UserWidget.AddToViewport` _output_get 0)
      (`Widget.SetVisibility` (`self.Level12Part1`) "Visible")
      (set `PlayerController.bShowMouseCursor` true (`GameplayStatics.GetPlayerController` 0)))))

(fn `UserConstructionScript`
  (`parent.UserConstructionScript`))