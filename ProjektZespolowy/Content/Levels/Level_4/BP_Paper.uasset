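; BP_Paper is an interactable paper in Level 4 that opens and closes the WBP_Level4PartIII UI.
; BeginInteraction checks for the first-person character, then uses a FlipFlop to alternate between open and closed.
; Opening sends a camera-adjust message with a hard-coded view, shows the mouse cursor and lazily creates the widget, which is cached for reuse.
; Closing releases the camera, collapses the widget and hides the cursor.
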(event `self.BeginInteraction`
  (bind _returnvalue (`GameplayStatics.GetPlayerCharacter` 0))
  (bind _returnvalue_2 (`GameplayStatics.GetPlayerController` 0))
  (bind _asbp_first_person_character (cast `/Game/FirstPerson/Blueprints/BP_FirstPersonCharacter` _returnvalue))
  (`/Engine/EditorBlueprintResources/StandardMacros.FlipFlop`
    (:`A`
      (message `/Game/Interactions/BPI_Interaction.Camera_Adjust_On` _returnvalue (`KismetMathLibrary.MakeVector` 4.109033 421.89364 150.0) (`KismetMathLibrary.MakeRotator` -57.3 -90.0 0.0))
      (bind _level_4part_3 (`self.Level 4Part 3`)
        (:`then`
          (`Widget.SetVisibility` _level_4part_3 "Visible")
          (set `PlayerController.bShowMouseCursor` true _returnvalue_2))
        (:`else`
          (bind _returnvalue_3 (`|CreateWidget` "/Game/LevelWidgets/LEVEL4/WBP_Level4PartIII.WBP_Level4PartIII_C" _returnvalue_2))
          (bind _output_get (set `self.Level 4Part 3` _returnvalue_3))
          (`UserWidget.AddToViewport` _output_get 0)
          (`Widget.SetVisibility` _level_4part_3 "Visible")
          (set `PlayerController.bShowMouseCursor` true _returnvalue_2))))
    (:`B`
      (message `/Game/Interactions/BPI_Interaction.Camera_Adjust_Off` _returnvalue)
      (`Widget.SetVisibility` _level_4part_3 "Collapsed")
      (set `PlayerController.bShowMouseCursor` false _returnvalue_2))))

(fn `UserConstructionScript`)