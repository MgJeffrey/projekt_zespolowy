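; BP_Makieta is a Level 1 interactable that toggles a top-down view and a cables UI for the player.
; A FlipFlop on BeginInteraction alternates between sending the player character a fixed overhead camera adjustment and releasing it.
; The first activation lazily creates and caches WBP_Cables; later toggles switch its visibility along with the mouse cursor.
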(event `self.BeginInteraction`
  (bind _returnvalue (`GameplayStatics.GetPlayerCharacter` 0))
  (bind _returnvalue_2 (`GameplayStatics.GetPlayerController` 0))
  ; Interaction
  (`/Engine/EditorBlueprintResources/StandardMacros.FlipFlop`
    (:`A`
      (message `/Game/Interactions/BPI_Interaction.Camera_Adjust_On` _returnvalue (`KismetMathLibrary.MakeVector` 194.140054 240.0 150.0) (`KismetMathLibrary.MakeRotator` 0.0 -90.0))
      (bind _cableswidget (`self.CablesWIdget`)
        (:`then`
          (`Widget.SetVisibility` _cableswidget "Visible")
          (set `PlayerController.bShowMouseCursor` true _returnvalue_2))
        (:`else`
          (bind _returnvalue_3 (`|CreateWidget` "/Game/LevelWidgets/WBP_Cables.WBP_Cables_C" _returnvalue_2))
          (bind _output_get (set `self.CablesWIdget` _returnvalue_3))
          (`UserWidget.AddToViewport` _output_get 0)
          (`Widget.SetVisibility` (`self.CablesWIdget`) "Visible")
          (`Widget.SetVisibility` _cableswidget "Visible")
          (set `PlayerController.bShowMouseCursor` true _returnvalue_2))))
    (:`B`
      (message `/Game/Interactions/BPI_Interaction.Camera_Adjust_Off` _returnvalue)
      (`Widget.SetVisibility` _cableswidget "Collapsed")
      (set `PlayerController.bShowMouseCursor` false _returnvalue_2))))

(fn `UserConstructionScript`)