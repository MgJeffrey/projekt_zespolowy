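; BP_Tablica is an interactable board that opens the two-part Level 4 UI.
; BeginInteraction alternates via FlipFlop between focusing the camera on a fixed view, hiding the first-person mesh, and restoring both.
; Each opening creates fresh Part I and Part II widgets, shows Part II if Part I's Passed flag is set, otherwise Part I, and enables the cursor.
; Closing collapses the widget selected by that flag and hides the cursor.
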(event `self.BeginInteraction`
  (bind _returnvalue (`GameplayStatics.GetPlayerCharacter` 0))
  (bind _returnvalue_2 (`GameplayStatics.GetPlayerController` 0))
  (bind _returnvalue_3 (`GameplayStatics.GetPlayerController` 0))
  (bind _level_4part_1 (`self.Level 4Part 1`))
  (bind _asbp_first_person_character (cast `/Game/FirstPerson/Blueprints/BP_FirstPersonCharacter` _returnvalue))
  (`/Engine/EditorBlueprintResources/StandardMacros.FlipFlop`
    (:`A`
      (message `/Game/Interactions/BPI_Interaction.Camera_Adjust_On` _returnvalue (`KismetMathLibrary.MakeVector` -10.0 400.0 200.0) (`KismetMathLibrary.MakeRotator` 0.0 0.0 90.0))
      (bind _firstpersonmesh (`/Game/FirstPerson/Blueprints/BP_FirstPersonCharacter.FirstPersonMesh` _asbp_first_person_character))
      (`SceneComponent.SetVisibility` _firstpersonmesh false false)
      (bind _returnvalue_4 (`|CreateWidget` "/Game/LevelWidgets/LEVEL4/WBP_Level4PartI.WBP_Level4PartI_C" _returnvalue_2))
      (bind _output_get (set `self.Level 4Part 1` _returnvalue_4))
      (`UserWidget.AddToViewport` _output_get 0)
      (`Widget.SetVisibility` _returnvalue_4 "Collapsed")
      (bind _returnvalue_5 (`|CreateWidget` "/Game/LevelWidgets/LEVEL4/WBP_Level4PartII.WBP_Level4PartII_C" _returnvalue_2))
      (bind _output_get_2 (set `self.Level 4Part 2` _returnvalue_5))
      (`UserWidget.AddToViewport` _output_get_2 0)
      (`Widget.SetVisibility` _returnvalue_5 "Collapsed")
      (if (`/Game/LevelWidgets/LEVEL4/WBP_Level4PartI.Passed?` (`self.Level 4Part 1`))
        (`Widget.SetVisibility` (`self.Level 4Part 2`) "Visible")
        (set `PlayerController.bShowMouseCursor` true (`GameplayStatics.GetPlayerController` 0))
        (else
          (`Widget.SetVisibility` (`self.Level 4Part 1`) "Visible")
          (set `PlayerController.bShowMouseCursor` true (`GameplayStatics.GetPlayerController` 0)))))
    (:`B`
      (message `/Game/Interactions/BPI_Interaction.Camera_Adjust_Off` _returnvalue)
      (`SceneComponent.SetVisibility` _firstpersonmesh true false)
      (if (`/Game/LevelWidgets/LEVEL4/WBP_Level4PartI.Passed?` _level_4part_1)
        (`Widget.SetVisibility` (`self.Level 4Part 2`) "Collapsed")
        (set `PlayerController.bShowMouseCursor` false _returnvalue_3)
        (else
          (`Widget.SetVisibility` _level_4part_1 "Collapsed")
          (set `PlayerController.bShowMouseCursor` false _returnvalue_3))))))

(fn `UserConstructionScript`)