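; Level 8 component that decides which operating system screen appears when the in-game PC starts.
; StartPC shows Windows only with HavePen and WinPenPlugged set, picking Windows2 if WindowsInstalled or Windows1 otherwise; all other cases show Linux.
; Windows1 and Linux are created only when not already valid, then enable the cursor and Game-and-UI input.
; Windows2 is created on each such call without changing cursor or input mode.
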(event `Start PC`
  (bind _returnvalue (`GameplayStatics.GetPlayerController` 0))
  (bind _returnvalue_2 (`GameplayStatics.GetPlayerController` 0))
  (if (`self.havePen?`)
    (if (`self.winPenPlugged?`)
      (if (`self.windowsInstalled?`)
        (bind _returnvalue_3 (`|CreateWidget` "/Game/Levels/Level_8/WIndows/WBP_Windows2.WBP_Windows2_C" (`GameplayStatics.GetPlayerController` 0)))
        (bind _output_get (set `self.Windows2` _returnvalue_3))
        (`UserWidget.AddToViewport` _output_get 0)
        (else
          (`self.Windows1`
            (:`then`)
            (:`else`
              (bind _returnvalue_4 (`|CreateWidget` "/Game/Levels/Level_8/WIndows/WBP_Windows1.WBP_Windows1_C" (`GameplayStatics.GetPlayerController` 0)))
              (bind _output_get_2 (set `self.Windows1` _returnvalue_4))
              (`UserWidget.AddToViewport` _output_get_2 0)
              (set `PlayerController.bShowMouseCursor` true _returnvalue)
              (`WidgetBlueprintLibrary.SetInputMode_GameAndUIEx` _returnvalue null "DoNotLock" false)))))
      (else
        (`self.Linux` :!label _label
          (:`then`)
          (:`else`
            (bind _returnvalue_5 (`|CreateWidget` "/Game/Levels/Level_8/Linux/WBP_SystemLinux.WBP_SystemLinux_C" (`GameplayStatics.GetPlayerController` 0)))
            (bind _output_get_3 (set `self.Linux` _returnvalue_5))
            (`UserWidget.AddToViewport` _output_get_3 0)
            (set `PlayerController.bShowMouseCursor` true _returnvalue_2)
            (`WidgetBlueprintLibrary.SetInputMode_GameAndUIEx` _returnvalue_2 null "DoNotLock" false)))))
    (else
      (goto _label))))