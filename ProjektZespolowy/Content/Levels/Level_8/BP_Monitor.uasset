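; BP_Monitor is an interactable monitor in Level 8 that moves the player's camera to a fixed close-up view.
; Each interaction alternates through a FlipFlop between the player character's camera adjust on and off messages, with a hard-coded location and rotation.
; BeginPlay creates a WBP_SystemLinux widget but neither stores nor displays it.
; Disconnected leftover logic would show or hide a WBP_Cables widget and the mouse cursor.
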(event `self.ReceiveBeginPlay`
  (`|CreateWidget` "/Game/Levels/Level_8/Linux/WBP_SystemLinux.WBP_SystemLinux_C"))

(event `self.BeginInteraction`
  (bind _returnvalue (`GameplayStatics.GetPlayerCharacter` 0))
  (`/Engine/EditorBlueprintResources/StandardMacros.FlipFlop`
    (:`A`
      (message `/Game/Interactions/BPI_Interaction.Camera_Adjust_On` _returnvalue (`KismetMathLibrary.MakeVector` 257.650106 712.683307 156.941589) (`KismetMathLibrary.MakeRotator` 0.0 -5.0 180.0)))
    (:`B`
      (message `/Game/Interactions/BPI_Interaction.Camera_Adjust_Off` _returnvalue))))

(fn `UserConstructionScript`)